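; BP_Cube is a placeholder enemy cube tracked by IvanGamemode's enemy count.
; On BeginPlay it increments EnemiesAlive on the game mode.
; When its cube component is hit by BP_TestCharacter, it decrements the count, calls CheckEnemiesLeft and destroys itself.
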(event OnComponentHit(Cube)
  (params (HitComponent :type Primitive%20Component%20Object%20Reference) (OtherActor :type Actor%20Object%20Reference) (OtherComp :type Primitive%20Component%20Object%20Reference) (NormalImpulse :type Vector :default "0, 0, 0") (Hit :type Hit%20Result%20Structure%20%28by%20ref%29))
  (Utilities|Casting|CastToBP_TestCharacter OtherActor)
  (bind _asivan_gamemode (Utilities|Casting|CastToIvanGamemode (Game|GetGameMode)))
  (Math|Integer|DecrementInt (Variables|/Game/Ivan/IvanGamemode.IvanGamemode_C|GetenemiesAlive _asivan_gamemode)
    (:%20%20
      (Default|CheckEnemiesLeft _asivan_gamemode)
      (Actor|DestroyActor))))

(event EventBeginPlay
  (bind _asivan_gamemode (Utilities|Casting|CastToIvanGamemode (Game|GetGameMode)))
  (Math|Integer|IncrementInt (Variables|/Game/Ivan/IvanGamemode.IvanGamemode_C|GetenemiesAlive _asivan_gamemode)))

(fn ConstructionScript)